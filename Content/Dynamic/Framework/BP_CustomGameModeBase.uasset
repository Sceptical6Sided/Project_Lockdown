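; Game mode that runs a match countdown and spawns a pawn for each joining player.
; On BeginPlay it copies the remaining time to BP_CustomGameStateBase and starts a looping timer.
; Each tick decrements the time and mirrors it to the game state, clearing the timer once it drops below zero.
; PostLogin spawns a BP_Characterbase_0 at a found player start and possesses it with the new controller.
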(event `self.ReceiveBeginPlay`
  (bind _asbp_custom_game_state_base (cast `/Game/Dynamic/Framework/BP_CustomGameStateBase` (`GameplayStatics.GetGameState`)))
  (set `/Game/Dynamic/Framework/BP_CustomGameStateBase.RemainingTimer` (`self.RemainingTime`) _asbp_custom_game_state_base)
  (`KismetSystemLibrary.K2_SetTimer` null "OnTimerTick" (`self.TimerInterval`) true))

(event `self.K2_PostLogin`
  (params (NewPlayer :type "PlayerController Object Reference"))
  (bind _returnvalue (`|SpawnActorFromClass` "/Game/Dynamic/Framework/BP_Characterbase_0.BP_Characterbase_0_C" (`self.GetTransform` (`self.K2_FindPlayerStart` NewPlayer "Player")) "Undefined" "MultiplyWithRoot" null null))
  (`Controller.Possess` NewPlayer _returnvalue))

(fn `OnTimerTick`
  (if (>= (`self.RemainingTime`) 0)
    (set `self.RemainingTime` (- (`self.RemainingTime`) 1))
    (bind _asbp_custom_game_state_base (cast `/Game/Dynamic/Framework/BP_CustomGameStateBase` (`GameplayStatics.GetGameState`)))
    (set `/Game/Dynamic/Framework/BP_CustomGameStateBase.RemainingTimer` (`self.RemainingTime`) _asbp_custom_game_state_base)
    (else
      (`KismetSystemLibrary.K2_ClearTimer` null "OnTimerTick"))))

(fn `UserConstructionScript`)